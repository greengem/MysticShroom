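; Debug trigger actor that unlocks the shrink ability on the player's third-person character.
; On any actor overlap it gets player 0's character and, if shrink is not yet enabled, sets the flag and fires the OnShrinkEnabled dispatcher.
; It then copies its checkpoint progress string to the character and its save object and saves to the character's slot.
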(event Collision|EventActorBeginOverlap
  (params (OtherActor :type Actor%20Object%20Reference))
  (bind _checkpoint_progress_string (Variables|Default|GetCheckpoint%20Progress%20String))
  (bind _asbp_third_person_character (Utilities|Casting|CastToBP_ThirdPersonCharacter (Game|GetPlayerCharacter 0)))
  (bind _output_get (Variables|Default|SetAs%20BP%20Third%20Person%20Character _asbp_third_person_character))
  (if (not (Variables|/Game/ThirdPerson/Blueprints/BP_ThirdPersonCharacter.BP_ThirdPersonCharacter_C|GetAbility_Shrink _output_get))
    (Variables|/Game/ThirdPerson/Blueprints/BP_ThirdPersonCharacter.BP_ThirdPersonCharacter_C|SetAbility_Shrink (Variables|Default|GetAs%20BP%20Third%20Person%20Character) true)
    (Default|CallOnShrinkEnabled)
    (if true
      (Variables|/Game/ThirdPerson/Blueprints/BP_ThirdPersonCharacter.BP_ThirdPersonCharacter_C|SetCheckpointProgressString (Variables|Default|GetAs%20BP%20Third%20Person%20Character) _checkpoint_progress_string)
      (Variables|/Game/ThirdPerson/Maps/BP_Save.BP_Save_C|SetCheckpointProgressString (Variables|/Game/ThirdPerson/Blueprints/BP_ThirdPersonCharacter.BP_ThirdPersonCharacter_C|GetBP_Save (Variables|Default|GetAs%20BP%20Third%20Person%20Character)) _checkpoint_progress_string)
      (SaveGame|SaveGametoSlot (Variables|/Game/ThirdPerson/Blueprints/BP_ThirdPersonCharacter.BP_ThirdPersonCharacter_C|GetBP_Save (Variables|Default|GetAs%20BP%20Third%20Person%20Character)) (Variables|/Game/ThirdPerson/Blueprints/BP_ThirdPersonCharacter.BP_ThirdPersonCharacter_C|GetSaveName (Variables|Default|GetAs%20BP%20Third%20Person%20Character))))))

(fn ConstructionScript)