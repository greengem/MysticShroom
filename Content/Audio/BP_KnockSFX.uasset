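; BP_KnockSFX is an actor Blueprint that plays impact sounds when it takes a hard hit.
; On BeginPlay it binds its hit event, which prints a debug string and filters for strong impulses against other actors.
; The hit's physical material selects a sound from the PhysMat map, played at the impact location with impulse-scaled volume and random pitch.
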(event Custom|HitEvent
  (params (SelfActor :type Actor%20Object%20Reference) (OtherActor :type Actor%20Object%20Reference) (NormalImpulse :type Vector) (Hit :type Hit%20Result%20Structure%20%28by%20ref%29))
  (bind (_bblockinghit _binitialoverlap _time _distance _location _impactpoint _normal _impactnormal _physmat _hitactor) (Collision|BreakHitResult Hit))
  (bind _returnvalue (Math|Vector|VectorLength NormalImpulse))
  (bind _phys_mat (Variables|Default|GetPhys%20Mat))
  (bind (_value _returnvalue_2) (Utilities|Map|Find _phys_mat _physmat))
  (Development|PrintString "Hello")
  (if (> _returnvalue 4e+03)
    (if (!= _hitactor self)
      (Variables|Default|SetForce (Math|Float|MapRangeClamped _returnvalue 0.0 5e+03 0.0 (Variables|Default|GetVolume)))
      (bind _output_get (Variables|Default|SetHit%20Location _location))
      (if _returnvalue_2
        (Audio|PlaySoundatLocation _value _output_get "0, 0, 0" (Variables|Default|GetForce) (Math|Random|RandomFloatinRange 0.0 1.0) 0.0 0 0 0 0)))))

(event EventBeginPlay
  (Collision|BindEventtoOnActorHit (delegate Custom|HitEvent)))

(fn ConstructionScript)