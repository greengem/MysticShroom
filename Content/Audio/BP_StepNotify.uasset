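; Animation notify that plays surface-dependent footstep sounds.
; It traces 100 units along the owner's negative up vector against complex collision and switches on the hit's surface type: Rock, Wood, Platform (layering rock and platform sounds), or grass by default.
; Sounds play at world origin rather than at the owner, with debug trace and surface-name prints left on.
; The branch is hardwired true, so "No Material" never prints.
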(fn ReceivedNotify
  (params (MeshComp :type Skeletal%20Mesh%20Component%20Object%20Reference) (Animation :type Anim%20Sequence%20Base%20Object%20Reference) (EventReference :type Anim%20Notify%20Event%20Reference%20Structure%20%28by%20ref%29))
  (bind _returnvalue (Components|GetOwner MeshComp))
  (bind _returnvalue_2 (Transformation|GetActorLocation _returnvalue))
  (bind _outhit (Collision|LineTraceByChannel _returnvalue_2 (+ _returnvalue_2 (* (Transformation|GetActorUpVector _returnvalue) -1e+02)) "TraceTypeQuery1" true 0 "ForDuration"))
  (if true
    (switch Utilities|FlowControl|Switch|SwitchonEPhysicalSurface (Collision|GetSurfaceType _outhit)
      (:SurfaceType_Default
        (Audio|PlaySoundatLocation "/Game/Audio/MS_GrassStep.MS_GrassStep" "0, 0, 0" "0, 0, 0" 1.0 1.0 0.0 0 0 0 0)
        (Development|PrintString "Grass"))
      (:SurfaceType2
        (Audio|PlaySoundatLocation "/Game/Audio/MS_RockStep.MS_RockStep" "0, 0, 0" "0, 0, 0" 1.0 1.0 0.0 0 0 0 0)
        (Development|PrintString "Rock"))
      (:SurfaceType3
        (Audio|PlaySoundatLocation "/Game/Audio/MS_WoodStep.MS_WoodStep" "0, 0, 0" "0, 0, 0" 1.0 1.0 0.0 0 0 0 0)
        (Development|PrintString "Wood"))
      (:SurfaceType4
        (Audio|PlaySoundatLocation "/Game/Audio/MS_RockStep.MS_RockStep" "0, 0, 0" "0, 0, 0" 1.0 1.0 0.0 0 0 0 0)
        (Audio|PlaySoundatLocation "/Game/Audio/MS_PlatformStep.MS_PlatformStep" "0, 0, 0" "0, 0, 0" 1.0 1.0 0.0 0 0 0 0)
        (Development|PrintString "Platform")))
    (return false)
    (else
      (Development|PrintString "No Material"))))