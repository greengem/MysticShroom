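; Trigger actor that changes the music when the BP_ThirdPersonCharacter begins overlapping it.
; It loops over its Sections enum array, converts each entry's name into a trigger parameter on MSMusicRedesign, and prints debug messages.
; End overlap does nothing, and the hard-coded per-instrument trigger, reset and index calls are disconnected, so they never run.
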(event Collision|EventActorEndOverlap
  (params (OtherActor :type Actor%20Object%20Reference))
  (Utilities|FlowControl|Sequence))

(event Collision|EventActorBeginOverlap
  (params (OtherActor :type Actor%20Object%20Reference))
  (Utilities|Casting|CastToBP_ThirdPersonCharacter OtherActor)
  (Development|PrintString "OVERLAP")
  (for _array_element (Variables|Default|GetSections)
    (Class|AudioParameterControllerInterface|SetTriggerParameter (Variables|Default|GetMS_MusicRedesign) (Utilities|String|StringToName (Utilities|String|EnumtoString _array_element)))
    (Development|PrintString (Utilities|String|ToString(Name) (Utilities|String|StringToName (Utilities|String|EnumtoString _array_element))) true true "(R=0.000000,G=0.660000,B=1.000000,A=1.000000)" 2e+01)))

(fn ConstructionScript)