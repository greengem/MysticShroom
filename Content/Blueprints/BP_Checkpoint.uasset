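; BP_Checkpoint is a trigger actor that advances and saves the player's checkpoint progress in a fixed order.
; When a BP_ThirdPersonCharacter overlaps its box, it sets the character's CPCurent to TargetCP only if that value equals PrevCP, so checkpoints register in sequence.
; It then writes the value into the character's save object, saves it to slot, and shows a WB_Checkpoint widget for a few seconds.
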(event OnComponentBeginOverlap(Box)
  (params (OverlappedComponent :type Primitive%20Component%20Object%20Reference) (OtherActor :type Actor%20Object%20Reference) (OtherComp :type Primitive%20Component%20Object%20Reference) (OtherBodyIndex :type Integer) (bFromSweep :type Boolean) (SweepResult :type Hit%20Result%20Structure%20%28by%20ref%29))
  (bind _asbp_third_person_character (Utilities|Casting|CastToBP_ThirdPersonCharacter OtherActor))
  (if (Utilities|Enum|Equal(Enum) (Variables|/Game/ThirdPerson/Blueprints/BP_ThirdPersonCharacter.BP_ThirdPersonCharacter_C|GetCPCurent _asbp_third_person_character) (Variables|Default|GetPrevCP))
    (bind _output_get (Variables|/Game/ThirdPerson/Blueprints/BP_ThirdPersonCharacter.BP_ThirdPersonCharacter_C|SetCPCurent _asbp_third_person_character (Variables|Default|GetTargetCP)))
    (Variables|/Game/ThirdPerson/Maps/BP_Save.BP_Save_C|SetSaveGameCheckpoint (Variables|/Game/ThirdPerson/Blueprints/BP_ThirdPersonCharacter.BP_ThirdPersonCharacter_C|GetBP_Save _asbp_third_person_character) _output_get)
    (SaveGame|SaveGametoSlot (Variables|/Game/ThirdPerson/Blueprints/BP_ThirdPersonCharacter.BP_ThirdPersonCharacter_C|GetBP_Save _asbp_third_person_character) (Variables|/Game/ThirdPerson/Blueprints/BP_ThirdPersonCharacter.BP_ThirdPersonCharacter_C|GetSaveName _asbp_third_person_character))
    (bind _returnvalue (UserInterface|CreateWidget "/Game/UI/HUD/WB_Checkpoint.WB_Checkpoint_C"))
    (UserInterface|Viewport|AddtoViewport _returnvalue 0)
    (Utilities|FlowControl|Delay 5.0)
    (Widget|RemovefromParent _returnvalue)))

(fn ConstructionScript)