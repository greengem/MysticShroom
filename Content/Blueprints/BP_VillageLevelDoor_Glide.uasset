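; Village level door, apparently for the Glide level, that opens once the player has progressed far enough.
; Shortly after BeginPlay it reads the player character's current checkpoint and opens at once if Level 1 is complete or later.
; For earlier checkpoints it binds to the Teleport_Jump teleporter's used event and opens when the matching door value arrives.
; Opening instantly drops the actor below its position, with no animation.
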(event Custom|CustomEvent
  (params (DoorToUnlock :type E_Doors%20Enum :default "NewEnumerator0"))
  (if (Utilities|Enum|Equal(Enum) DoorToUnlock "NewEnumerator2")
    (CallFunction|OpenDoor)))

(event EventBeginPlay
  (Utilities|FlowControl|Delay 0.2)
  (bind _asbp_third_person_character (Utilities|Casting|CastToBP_ThirdPersonCharacter (Game|GetPlayerCharacter 0)))
  (switch Utilities|FlowControl|Switch|SwitchonE_Checkpoints (Variables|/Game/ThirdPerson/Blueprints/BP_ThirdPersonCharacter.BP_ThirdPersonCharacter_C|GetCPCurent _asbp_third_person_character)
    (:NewEnumerator11
      (bind _outactors (Actor|GetAllActorsOfClasswithTag "/Game/Blueprints/Portal/BP_Teleport.BP_Teleport_C" "Teleport_Jump" :!label _label))
      (EventDispatchers|BindEventtoTelportUsed (Utilities|Array|Get(acopy) _outactors) (delegate Custom|CustomEvent)))
    (:NewEnumerator12
      (goto _label))
    (:NewEnumerator13
      (goto _label))
    (:NewEnumerator14
      (goto _label))
    (:NewEnumerator15
      (goto _label))
    (:NewEnumerator16
      (CallFunction|OpenDoor :!label _label_2))
    (:NewEnumerator17
      (goto _label_2))
    (:NewEnumerator18
      (goto _label_2))
    (:NewEnumerator19
      (goto _label_2))
    (:NewEnumerator20
      (goto _label_2))
    (:NewEnumerator21
      (goto _label_2))
    (:NewEnumerator22
      (goto _label_2))))

(fn ConstructionScript)

(fn OpenDoor
  (bind _returnvalue (Transformation|GetActorLocation))
  (Transformation|SetActorLocation (Math|Vector|MakeVector (.x _returnvalue) (.y _returnvalue) (- (.z _returnvalue) 5e+02)) false false))