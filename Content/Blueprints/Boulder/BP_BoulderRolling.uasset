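; BP_BoulderRolling is a physics boulder hazard that kills the third-person player on overlap, then opens MainLevel after a delay.
; Construction picks a random sphere material, and a timer destroys the boulder after a fixed lifetime.
; Hits above a speed threshold track impact height, playing an attached collision sound on the first impact and after large drops, throttled by a resetting DoOnce.
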(event OnComponentBeginOverlap(Sphere1)
  (params (OverlappedComponent :type Primitive%20Component%20Object%20Reference) (OtherActor :type Actor%20Object%20Reference) (OtherComp :type Primitive%20Component%20Object%20Reference) (OtherBodyIndex :type Integer) (bFromSweep :type Boolean) (SweepResult :type Hit%20Result%20Structure%20%28by%20ref%29))
  (bind _asbp_third_person_character (Utilities|Casting|CastToBP_ThirdPersonCharacter OtherActor))
  (Default|KillPlayer _asbp_third_person_character)
  (Utilities|FlowControl|Delay 4.0)
  (Game|OpenLevel(byName) "MainLevel"))

(event OnComponentHit(Sphere)
  (params (HitComponent :type Primitive%20Component%20Object%20Reference) (OtherActor :type Actor%20Object%20Reference) (OtherComp :type Primitive%20Component%20Object%20Reference) (NormalImpulse :type Vector :default "0, 0, 0") (Hit :type Hit%20Result%20Structure%20%28by%20ref%29))
  ;[1 1 1] Speed of Object. IF above certain threshold
  (bind _returnvalue (Physics|GetPhysicsLinearVelocity (Variables|Default|GetSphere) "None"))
  (if (<= 3e+01 (Math|Vector|VectorLength (Math|Vector|MakeVector (.x _returnvalue) (.y _returnvalue) (.z _returnvalue))))
    (Utilities|FlowControl|Sequence
      (:then_0
        ;[1 1 1] Triggers SFX with Prev Value
        (Utilities|FlowControl|DoOnce false
          (:Completed
            ;[1 1 1] Actual Audio being played when Bools have been met
            (Utilities|FlowControl|DoOnce false :!label _label
              (:Completed
                (Audio|SpawnSoundAttached "/Game/Audio/MS_Collision.MS_Collision" (Variables|Default|GetSphere) "None" "0, 0, 0" "0, 0, 0" "KeepRelativeOffset" false 1.0 1.0 0.0 "/Game/Audio/Attenuation/SA_Collision.SA_Collision" 0)
                (Utilities|FlowControl|Delay 0.7)
                (goto _label Reset))))))
      (:then_1
        ;[1 1 1] Set Current hit to previous hit and update Current hit location.
        (Variables|Default|SetPrev%20Hit (Variables|Default|GetCurrent%20Hit))
        (Variables|Default|SetCurrent%20Hit (Transformation|GetWorldLocation (Variables|Default|GetSphere)))
        ;[1 1 1] IF the "Current Hit" subtracted with "Prev Hit" is less than or equal to. ABS node for constant positive value. ABS value divided by 100 to simplify readability.
        (if (>= (/ (Math|Float|Absolute(Float) (.z (- (Variables|Default|GetCurrent%20Hit) (Variables|Default|GetPrev%20Hit)))) 1e+02) 12.0)
          ;[1 1 1] IF the subtracted Z vector between "Current Hit" and "Prev Hit" is below 0. This function is used to see if the object is going up or down in Z value.
          (if (> 0.0 (- (.z (Variables|Default|GetCurrent%20Hit)) (.z (Variables|Default|GetPrev%20Hit))))
            (goto _label)))))))

(event EventBeginPlay
  (Utilities|Time|SetTimerbyFunctionName 0 "DestroyBoulder" 4e+01))

(fn ConstructionScript
  (Rendering|Material|SetMaterial (Variables|Default|GetSphere) 0 (.OutItem (Utilities|Array|Random (Variables|Default|GetMaterialVar)))))

(fn DestroyBoulder
  (Actor|DestroyActor))