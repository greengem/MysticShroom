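; Boulder spawner actor that keeps spawning rolling boulders (BP_BoulderRolling) around its own location.
; On BeginPlay it starts a looping timer whose interval is randomized once, so each instance keeps its own fixed spawn rhythm of a few seconds.
; Each tick of the timer calls SpawnBoulder, which adds a random offset from the SpawnPos array to the actor's location to place the new boulder.
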(event Custom|SpawnBoulders
  (CallFunction|SpawnBoulder))

(event EventBeginPlay
  (Utilities|Time|SetTimerbyEvent (delegate Custom|SpawnBoulders) (Math|Random|RandomFloatinRange 1.0 5.0) true))

(fn ConstructionScript)

(fn SpawnBoulder
  (bind _returnvalue (Transformation|GetActorTransform))
  (bind _spawnpos (Variables|Default|GetSpawnPos))
  (bind _outitem (Utilities|Array|Random _spawnpos))
  (Game|SpawnActorfromClass "/Game/Blueprints/Boulder/BP_BoulderRolling.BP_BoulderRolling_C" (Math|Transform|MakeTransform (Math|Vector|MakeVector (+ (.x _outitem) (.x (.location _returnvalue))) (+ (.y _outitem) (.y (.location _returnvalue))) (+ (.z _outitem) (.z (.location _returnvalue)))) "0, 0, 0" "1.000000,1.000000,1.000000") "Undefined" "MultiplyWithRoot" 0 0))