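; Launch pad actor for the cloud platforms that boosts the third-person character upward when it overlaps the pad's box.
; On overlap it removes the character's gliding gameplay tag, then calls LaunchCharacter with a vertical velocity added to the current one.
; It records the pad's index and feeds it to the bounce MetaSound as a semitone parameter before playing, so the index sets the sound's pitch.
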(event OnComponentBeginOverlap(Box)
  (params (OverlappedComponent :type Primitive%20Component%20Object%20Reference) (OtherActor :type Actor%20Object%20Reference) (OtherComp :type Primitive%20Component%20Object%20Reference) (OtherBodyIndex :type Integer) (bFromSweep :type Boolean) (SweepResult :type Hit%20Result%20Structure%20%28by%20ref%29))
  (bind _asbp_third_person_character (Utilities|Casting|CastToBP_ThirdPersonCharacter OtherActor))
  (GameplayTags|RemoveGameplayTag (Variables|/Game/ThirdPerson/Blueprints/BP_ThirdPersonCharacter.BP_ThirdPersonCharacter_C|GetAbilityTags _asbp_third_person_character) "(TagName=\"Ability.Glide.isGliding\")" :!class /Script/GameplayTags.BlueprintGameplayTagLibrary)
  (Character|LaunchCharacter _asbp_third_person_character "0.000000,0.000000,3000.000000" false false)
  (Variables|Default|SetLastJumpPadIndex (Variables|Default|GetJumpPadIndex))
  (Class|AudioParameterControllerInterface|SetTriggerParameter(Message) (Variables|Default|GetMS_PlatformBounce) "ZValueSemiTones")
  (Audio|Parameter|SetFloatParameter (Variables|Default|GetMS_PlatformBounce) "ZValueSemiTones" (Variables|Default|GetJumpPadIndex) :!class /Script/Engine.AudioComponent)
  (Audio|Components|Audio|Play (Variables|Default|GetMS_PlatformBounce) 0.0))

(fn ConstructionScript)