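; BP_Teleport is a portal that moves the player character to a target checkpoint when it enters the box.
; Overlap pauses movement, fades the camera to black, teleports via the character's checkpoint map, fades back and fires a used dispatcher.
; If the player's current checkpoint is the previous one, it advances and saves progress, briefly showing a checkpoint widget.
; A separate activation event chains timelines that ramp the Niagara spawn rate, vortex force, then light intensity.
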(event OnComponentBeginOverlap(Box)
  (params (OverlappedComponent :type Primitive%20Component%20Object%20Reference) (OtherActor :type Actor%20Object%20Reference) (OtherComp :type Primitive%20Component%20Object%20Reference) (OtherBodyIndex :type Integer) (bFromSweep :type Boolean) (SweepResult :type Hit%20Result%20Structure%20%28by%20ref%29))
  (bind _asbp_third_person_character (Utilities|Casting|CastToBP_ThirdPersonCharacter OtherActor))
  (bind _output_get (Variables|Default|SetAs%20BP%20Third%20Person%20Character _asbp_third_person_character))
  (Components|Activation|Deactivate (Variables|/Script/Engine.Character|GetCharacterMovement _output_get)) ; Disable Player controls temporarily
  (CameraFades|StartCameraFade :self (Game|GetPlayerCameraManager 0) :ToAlpha 1.0 :Duration 1.0 :bHoldWhenFinished true) ; Fade to Black
  (Utilities|FlowControl|Delay 1.2) ; Hold black screen for 1.2s
  (Transformation|SetActorLocationAndRotation (Variables|Default|GetAs%20BP%20Third%20Person%20Character) (.location (.Value (Utilities|Map|Find (Variables|/Game/ThirdPerson/Blueprints/BP_ThirdPersonCharacter.BP_ThirdPersonCharacter_C|GetCPEnum (Variables|Default|GetAs%20BP%20Third%20Person%20Character)) (Variables|Default|GetTargetCP)))) (.rotation (.Value (Utilities|Map|Find (Variables|/Game/ThirdPerson/Blueprints/BP_ThirdPersonCharacter.BP_ThirdPersonCharacter_C|GetCPEnum (Variables|Default|GetAs%20BP%20Third%20Person%20Character)) (Variables|Default|GetTargetCP))))) ; Teleport actor position
  (Components|Activation|Activate (Variables|/Script/Engine.Character|GetCharacterMovement _output_get) false) ; Re-enable player controls
  (CameraFades|StartCameraFade :self (Game|GetPlayerCameraManager 0) :FromAlpha 1.0 :Duration 1.0) ; Fade from black to viewport
  (Default|CallTelportUsed (Variables|Default|GetTargetDoor)) ; Call event dispatcher to notify other components that the portal was used
  (|UpdateCheckpointandSaveGame) ; Update player checkpoint progress and update the save game
)

(event Custom|ActivatePortalEvent
  (bind _niagaraeffect (Variables|Default|GetNiagaraEffect))
  (Components|Activation|Activate _niagaraeffect false)
  (bind _newtrack_0 (Timeline|Timeline_0 PlayFromStart)
    (:Update
      (Effects|Components|ParticleSystem|SetFloatParameter _niagaraeffect "SpawnRate" _newtrack_0))
    (:Finished
      (bind _newtrack_0_2 (Timeline|Timeline_1 PlayFromStart)
        (:Update
          (Effects|Components|ParticleSystem|SetFloatParameter _niagaraeffect "VortexForce" _newtrack_0_2))
        (:Finished
          (bind _newtrack_0_3 (Timeline|Timeline PlayFromStart)
            (:Update
              (Rendering|Components|Light|SetIntensity (Variables|Default|GetPointLight) _newtrack_0_3))))))))

(fn ConstructionScript)