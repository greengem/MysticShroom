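; BP_EndGameTrigger is a trigger zone that ends the game when the third-person player character overlaps its box.
; On overlap it deactivates the character's movement, switches input to UI only with a visible cursor and click events, and displays the WB_EndGameCredits widget.
; After a short delay it plays the MS_HereKitty sound in 2D.
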(event OnComponentBeginOverlap(Box)
  (params (OverlappedComponent :type Primitive%20Component%20Object%20Reference) (OtherActor :type Actor%20Object%20Reference) (OtherComp :type Primitive%20Component%20Object%20Reference) (OtherBodyIndex :type Integer) (bFromSweep :type Boolean) (SweepResult :type Hit%20Result%20Structure%20%28by%20ref%29))
  (bind _returnvalue (Game|GetPlayerController 0))
  (bind _asbp_third_person_character (Utilities|Casting|CastToBP_ThirdPersonCharacter OtherActor))
  (Components|Activation|Deactivate (Variables|/Script/Engine.Character|GetCharacterMovement _asbp_third_person_character))
  (Input|SetInputModeUIOnly _returnvalue 0 "DoNotLock" false)
  (Variables|/Script/Engine.PlayerController|SetbShowMouseCursor _returnvalue true)
  (Variables|/Script/Engine.PlayerController|SetbEnableClickEvents _returnvalue true)
  (bind _returnvalue_2 (UserInterface|CreateWidget "/Game/UI/HUD/WB_EndGameCredits.WB_EndGameCredits_C"))
  (UserInterface|Viewport|AddtoViewport _returnvalue_2 0)
  (Utilities|FlowControl|Delay 1.5)
  (Audio|PlaySound2D "/Game/Audio/MS_HereKitty.MS_HereKitty" 1.0 1.0 0.0 0 0))

(fn ConstructionScript)