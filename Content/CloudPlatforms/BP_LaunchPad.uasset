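; BP_LaunchPad is a cloud-platform launch pad that throws characters upward and plays a pitched bounce sound.
; When a Character overlaps its Box, LaunchCharacter applies a fixed vertical velocity, added to the character's existing velocity rather than overriding it.
; The pad then stores its JumpPadIndex as LastJumpPadIndex and feeds it to MSPlatformBounce as a semitone parameter, so the bounce pitch follows the pad's index.
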(event OnComponentBeginOverlap(Box)
  (params (OverlappedComponent :type Primitive%20Component%20Object%20Reference) (OtherActor :type Actor%20Object%20Reference) (OtherComp :type Primitive%20Component%20Object%20Reference) (OtherBodyIndex :type Integer) (bFromSweep :type Boolean) (SweepResult :type Hit%20Result%20Structure%20%28by%20ref%29))
  (bind _ascharacter (Utilities|Casting|CastToCharacter OtherActor))
  (Character|LaunchCharacter _ascharacter "0.000000,0.000000,3000.000000" false false)
  (Variables|Default|SetLastJumpPadIndex (Variables|Default|GetJumpPadIndex))
  (Class|AudioParameterControllerInterface|SetTriggerParameter(Message) (Variables|Default|GetMS_PlatformBounce) "ZValueSemiTones")
  (Audio|Parameter|SetFloatParameter (Variables|Default|GetMS_PlatformBounce) "ZValueSemiTones" (Variables|Default|GetJumpPadIndex) :!class /Script/Engine.AudioComponent)
  (Audio|Components|Audio|Play (Variables|Default|GetMS_PlatformBounce) 0.0))

(event EventBeginPlay)

(event Collision|EventActorBeginOverlap
  (params (OtherActor :type Actor%20Object%20Reference)))

(event EventTick
  (params (DeltaSeconds :type Float%20%28single-precision%29)))

(fn ConstructionScript)