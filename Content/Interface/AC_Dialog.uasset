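; Dialog component that feeds lines from its Dialog array to the player character, one per Speaking call.
; Speaking first checks CheckSpeakingMessage on the player and, only if it returns false, passes the current line and TextDelay to SpeakingMessage.
; It then advances CurrentDialog, wrapping to the first line after the last so the dialog repeats in order.
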(event Custom|Speaking
  (bind _returnvalue (Game|GetPlayerCharacter 0))
  (bind _dialog (Variables|Default|GetDialog))
  (bind _bspeaking (Class|BPISpeech|CheckSpeaking(Message) _returnvalue))
  (if (not _bspeaking)
    (Class|BPISpeech|Speaking(Message) _returnvalue (Utilities|Array|Get(acopy) _dialog (Variables|Default|GetCurrentDialog)) (Variables|Default|GetTextDelay))
    (bind _result (Math|Integer|IncrementInt (Variables|Default|GetCurrentDialog))
      (:%20%20
        (if (>= _result (Utilities|Array|Length _dialog))
          (Variables|Default|SetCurrentDialog 0))))))