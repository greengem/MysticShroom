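; Toadstool Tim NPC that plays a one-time, linear dialog with the player.
; Each Talk event advances TalkIndex through the Dialog array into a lazily created WB_Dialog widget, removing it and hiding the interact prompt after the last line.
; TriggerZone swaps the name for the prompt when BP_ThirdPersonCharacter enters with lines remaining, and restores the name on any end overlap.
; TalkIndex never resets here.
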(event OnComponentBeginOverlap(TriggerZone)
  (params (OverlappedComponent :type Primitive%20Component%20Object%20Reference) (OtherActor :type Actor%20Object%20Reference) (OtherComp :type Primitive%20Component%20Object%20Reference) (OtherBodyIndex :type Integer) (bFromSweep :type Boolean) (SweepResult :type Hit%20Result%20Structure%20%28by%20ref%29))
  ;[0 1 0.7393] Show E image above NPC
  (Utilities|Casting|CastToBP_ThirdPersonCharacter OtherActor)
  (if (< (Variables|Default|GetTalkIndex) (Utilities|Array|Length (Variables|Default|GetDialog)))
    (Rendering|SetVisibility (Variables|Default|GetInteractButton) true false)
    (Rendering|SetVisibility (Variables|Default|GetNPCName) false false)))

(event OnComponentEndOverlap(TriggerZone)
  (params (OverlappedComponent :type Primitive%20Component%20Object%20Reference) (OtherActor :type Actor%20Object%20Reference) (OtherComp :type Primitive%20Component%20Object%20Reference) (OtherBodyIndex :type Integer))
  ;[0 1 0.7393] Show E image above NPC
  (Rendering|SetVisibility (Variables|Default|GetInteractButton) false false)
  (Rendering|SetVisibility (Variables|Default|GetNPCName) true false))

(event EventTalk
  (params (NPC%20Name :type String))
  (Math|Integer|IncrementInt (Variables|Default|GetTalkIndex)
    (:%20%20
      (if (< (Variables|Default|GetTalkIndex) (Utilities|Array|Length (Variables|Default|GetDialog)))
        (Variables|Default|GetUI_Dialog
          (:then
            _)
          (:else
            (bind _returnvalue (UserInterface|CreateWidget "/Game/UI/HUD/WB_Dialog.WB_Dialog_C" (Game|GetPlayerController 0)))
            (bind _output_get (Variables|Default|SetUI_Dialog _returnvalue))
            (UserInterface|Viewport|AddtoViewport _output_get 0)))
        (Rendering|Components|TextRender|SetText (Variables|/Game/UI/HUD/WB_Dialog.WB_Dialog_C|GetTalkText (Variables|Default|GetUI_Dialog)) (Utilities|Text|ToText(String) (Utilities|Array|Get(acopy) (Variables|Default|GetDialog) (Variables|Default|GetTalkIndex))))
        (else
          (Widget|RemovefromParent (Variables|Default|GetUI_Dialog))
          (Rendering|SetVisibility (Variables|Default|GetInteractButton) false false))))))

(fn ConstructionScript)