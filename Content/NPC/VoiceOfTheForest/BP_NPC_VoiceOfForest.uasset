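; Forest voice NPC that plays a one-time intro dialogue when the player character overlaps its box.
; It deactivates the character's movement and steps through the Dialog array in a WB_Dialog widget on a looping timer.
; After the last line it removes the widget, activates the BP_Teleport tagged Teleport_Intro, restores movement after a short delay and marks itself used.
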(event OnComponentBeginOverlap(Box)
  (params (OverlappedComponent :type Primitive%20Component%20Object%20Reference) (OtherActor :type Actor%20Object%20Reference) (OtherComp :type Primitive%20Component%20Object%20Reference) (OtherBodyIndex :type Integer) (bFromSweep :type Boolean) (SweepResult :type Hit%20Result%20Structure%20%28by%20ref%29))
  (if (not (Variables|Default|GetisUsed))
    (bind _asbp_third_person_character (Utilities|Casting|CastToBP_ThirdPersonCharacter OtherActor))
    (bind _output_get (Variables|Default|SetCharacter%20Movement (Variables|/Script/Engine.Character|GetCharacterMovement _asbp_third_person_character)))
    (Components|Activation|Deactivate _output_get)
    (bind _outactors (Actor|GetAllActorsOfClasswithTag "/Game/Blueprints/Portal/BP_Teleport.BP_Teleport_C" "Teleport_Intro"))
    (Variables|Default|SetAs%20BP%20Teleport (Utilities|Array|Get(acopy) _outactors))
    (Math|Integer|IncrementInt (Variables|Default|GetDialogIndex)
      (:%20%20
        (CallFunction|Talk)
        (bind _returnvalue (Utilities|Time|SetTimerbyEvent (delegate Custom|SayMessages) 12.0 true))))))

(event Custom|SayMessages
  (Math|Integer|IncrementInt (Variables|Default|GetDialogIndex)
    (:%20%20
      (if (< (Variables|Default|GetDialogIndex) (Utilities|Array|Length (Variables|Default|GetDialog)))
        (CallFunction|Talk)
        (else
          (Utilities|Time|ClearandInvalidateTimerbyHandle (stale OnComponentBeginOverlap(Box) _returnvalue))
          (Widget|RemovefromParent (Variables|Default|GetWB%20Dialog))
          (Default|ActivatePortalEvent (Variables|Default|GetAs%20BP%20Teleport))
          (Utilities|FlowControl|Delay 1.0)
          (Components|Activation|Activate (Variables|Default|GetCharacter%20Movement) false)
          (Variables|Default|SetisUsed true))))))

(event EventTalk
  (params (NPC%20Name :type String))
  (Variables|Default|GetWB%20Dialog
    (:then
      _)
    (:else
      (bind _returnvalue (UserInterface|CreateWidget "/Game/UI/HUD/WB_Dialog.WB_Dialog_C" (Game|GetPlayerController 0)))
      (bind _output_get (Variables|Default|SetWB%20Dialog _returnvalue))
      (UserInterface|Viewport|AddtoViewport _output_get 0)))
  (Rendering|Components|TextRender|SetText (Variables|/Game/UI/HUD/WB_Dialog.WB_Dialog_C|GetTalkText (Variables|Default|GetWB%20Dialog)) (Utilities|Text|ToText(String) (Utilities|Array|Get(acopy) (Variables|Default|GetDialog) (Variables|Default|GetDialogIndex)))))

(fn ConstructionScript)