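; Portal actor that teleports the third-person character to a target checkpoint when it overlaps the trigger box.
; On overlap it pauses character movement, fades to black, moves the player to the transform from the character's checkpoint map, then fades back in.
; It then broadcasts a portal-used dispatcher with the door to unlock, and saves checkpoint progress only if the player's current checkpoint matches the expected previous one.
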(event OnComponentBeginOverlap(Box)
  (params (OverlappedComponent :type Primitive%20Component%20Object%20Reference) (OtherActor :type Actor%20Object%20Reference) (OtherComp :type Primitive%20Component%20Object%20Reference) (OtherBodyIndex :type Integer) (bFromSweep :type Boolean) (SweepResult :type Hit%20Result%20Structure%20%28by%20ref%29))
  (bind _asbp_third_person_character (Utilities|Casting|CastToBP_ThirdPersonCharacter OtherActor))
  (bind _output_get (Variables|Default|SetAs%20BP%20Third%20Person%20Character _asbp_third_person_character))
  (Components|Activation|Deactivate (Variables|/Script/Engine.Character|GetCharacterMovement _output_get)) ; Disable Player controls temporarily
  (CameraFades|StartCameraFade :self (Game|GetPlayerCameraManager 0) :ToAlpha 1.0 :Duration 1.0 :bHoldWhenFinished true) ; Fade to Black
  (Utilities|FlowControl|Delay 1.2) ; Hold black screen for 1.2s
  (Transformation|SetActorLocationAndRotation (Variables|Default|GetAs%20BP%20Third%20Person%20Character) (.location (.Value (Utilities|Map|Find (Variables|/Game/ThirdPerson/Blueprints/BP_ThirdPersonCharacter.BP_ThirdPersonCharacter_C|GetCheckpointsMap (Variables|Default|GetAs%20BP%20Third%20Person%20Character)) (Variables|Default|GetTargetCheckpoint)))) (.rotation (.Value (Utilities|Map|Find (Variables|/Game/ThirdPerson/Blueprints/BP_ThirdPersonCharacter.BP_ThirdPersonCharacter_C|GetCheckpointsMap (Variables|Default|GetAs%20BP%20Third%20Person%20Character)) (Variables|Default|GetTargetCheckpoint))))) ; Teleport actor position
  (Components|Activation|Activate (Variables|/Script/Engine.Character|GetCharacterMovement _output_get) false) ; Re-enable player controls
  (CameraFades|StartCameraFade :self (Game|GetPlayerCameraManager 0) :FromAlpha 1.0 :Duration 1.0) ; Fade from black to viewport
  (Default|CallTelportUsed (Variables|Default|GetDoor%20to%20Unlock)) ; Call event dispatcher to notify other components that the portal was used
  (|UpdateCheckpointandSaveGame) ; Update player checkpoint progress and update the save game
)

(fn ConstructionScript)