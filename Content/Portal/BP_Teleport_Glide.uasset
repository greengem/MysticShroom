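; Portal trigger that teleports the third-person character to checkpoint index 5 when it overlaps the box.
; On overlap it unlocks the village Dash level door, fires the Glide teleport-used call and grants the Dash ability.
; It advances checkpoint progress from 4 to 5 on the character, but always writes 5 to the save object before saving it to the character's slot.
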(event OnComponentBeginOverlap(Box)
  (params (OverlappedComponent :type Primitive%20Component%20Object%20Reference) (OtherActor :type Actor%20Object%20Reference) (OtherComp :type Primitive%20Component%20Object%20Reference) (OtherBodyIndex :type Integer) (bFromSweep :type Boolean) (SweepResult :type Hit%20Result%20Structure%20%28by%20ref%29))
  (bind _asbp_third_person_character (Utilities|Casting|CastToBP_ThirdPersonCharacter OtherActor))
  (Transformation|SetActorLocationAndRotation _asbp_third_person_character (.location (Utilities|Array|Get(acopy) (Variables|/Game/ThirdPerson/Blueprints/BP_ThirdPersonCharacter.BP_ThirdPersonCharacter_C|GetCheckpoints _asbp_third_person_character) 5)) (.rotation (Utilities|Array|Get(acopy) (Variables|/Game/ThirdPerson/Blueprints/BP_ThirdPersonCharacter.BP_ThirdPersonCharacter_C|GetCheckpoints _asbp_third_person_character) 5)))
  (bind _returnvalue (Actor|GetActorOfClass "/Game/_Debug/BP_VillageLevelDoor_Dash.BP_VillageLevelDoor_Dash_C"))
  (Variables|/Game/_Debug/BP_VillageLevelDoor_Dash.BP_VillageLevelDoor_Dash_C|SetisUnlocked _returnvalue true)
  (Default|CallTelportUsedGlide)
  (if (== (Variables|/Game/ThirdPerson/Blueprints/BP_ThirdPersonCharacter.BP_ThirdPersonCharacter_C|GetCheckpointProgress _asbp_third_person_character) 4)
    (Variables|/Game/ThirdPerson/Blueprints/BP_ThirdPersonCharacter.BP_ThirdPersonCharacter_C|SetCheckpointProgress _asbp_third_person_character 5))
  (Variables|/Game/ThirdPerson/Blueprints/BP_ThirdPersonCharacter.BP_ThirdPersonCharacter_C|SetAbility_Dash _asbp_third_person_character true)
  (Variables|/Game/ThirdPerson/Maps/BP_Save.BP_Save_C|SetCheckpointProgress (Variables|/Game/ThirdPerson/Blueprints/BP_ThirdPersonCharacter.BP_ThirdPersonCharacter_C|GetBP_Save _asbp_third_person_character) 5)
  (SaveGame|SaveGametoSlot (Variables|/Game/ThirdPerson/Blueprints/BP_ThirdPersonCharacter.BP_ThirdPersonCharacter_C|GetBP_Save _asbp_third_person_character) (Variables|/Game/ThirdPerson/Blueprints/BP_ThirdPersonCharacter.BP_ThirdPersonCharacter_C|GetSaveName _asbp_third_person_character)))

(fn ConstructionScript)