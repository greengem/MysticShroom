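; BP_Teleport_Jump is a portal trigger that teleports the third-person character to a stored checkpoint when it overlaps the Box.
; It moves and rotates the character to a fixed index in the character's Checkpoints array, then unlocks the village's Glide level door, found by class lookup.
; It also fires the TelportUsedJump dispatcher and advances CheckpointProgress only if the character is at the preceding step.
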(event OnComponentBeginOverlap(Box)
  (params (OverlappedComponent :type Primitive%20Component%20Object%20Reference) (OtherActor :type Actor%20Object%20Reference) (OtherComp :type Primitive%20Component%20Object%20Reference) (OtherBodyIndex :type Integer) (bFromSweep :type Boolean) (SweepResult :type Hit%20Result%20Structure%20%28by%20ref%29))
  (bind _asbp_third_person_character (Utilities|Casting|CastToBP_ThirdPersonCharacter OtherActor))
  (Transformation|SetActorLocationAndRotation _asbp_third_person_character (.location (Utilities|Array|Get(acopy) (Variables|/Game/ThirdPerson/Blueprints/BP_ThirdPersonCharacter.BP_ThirdPersonCharacter_C|GetCheckpoints _asbp_third_person_character) 3)) (.rotation (Utilities|Array|Get(acopy) (Variables|/Game/ThirdPerson/Blueprints/BP_ThirdPersonCharacter.BP_ThirdPersonCharacter_C|GetCheckpoints _asbp_third_person_character) 3)))
  (bind _returnvalue (Actor|GetActorOfClass "/Game/_Debug/BP_VillageLevelDoor_Glide.BP_VillageLevelDoor_Glide_C"))
  (Variables|/Game/_Debug/BP_VillageLevelDoor_Glide.BP_VillageLevelDoor_Glide_C|SetisUnlocked _returnvalue true)
  (Default|CallTelportUsedJump)
  (if (== (Variables|/Game/ThirdPerson/Blueprints/BP_ThirdPersonCharacter.BP_ThirdPersonCharacter_C|GetCheckpointProgress _asbp_third_person_character) 2)
    (Variables|/Game/ThirdPerson/Blueprints/BP_ThirdPersonCharacter.BP_ThirdPersonCharacter_C|SetCheckpointProgress _asbp_third_person_character 3)))

(fn ConstructionScript)