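; Procedural physics rope bridge that plays a creak sound when the third-person character steps into its trigger box.
; The construction script spawns a row of plank meshes along local Y, spaced by GapSize, and links each neighboring pair with a physics constraint.
; The first and last planks have physics simulation disabled to anchor the span.
; On overlap, it spawns MS_RopeBridge at the actor location and fires its CreakTrigger parameter.
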(event OnComponentBeginOverlap(AudioTriggerBox)
  (params (OverlappedComponent :type Primitive%20Component%20Object%20Reference) (OtherActor :type Actor%20Object%20Reference) (OtherComp :type Primitive%20Component%20Object%20Reference) (OtherBodyIndex :type Integer) (bFromSweep :type Boolean) (SweepResult :type Hit%20Result%20Structure%20%28by%20ref%29))
  (Utilities|Casting|CastToBP_ThirdPersonCharacter OtherActor)
  (bind _returnvalue (Audio|SpawnSoundatLocation "/Game/Audio/MS_RopeBridge.MS_RopeBridge" (Transformation|GetActorLocation) "0, 0, 0" 1.0 1.0 0.0 0 0))
  (Class|AudioParameterControllerInterface|SetTriggerParameter _returnvalue "CreakTrigger"))

(fn ConstructionScript
  (CallFunction|GeneratePlanks)
  (CallFunction|GenerateConstraints)
  (Physics|SetSimulatePhysics (Utilities|Array|Get(acopy) (Variables|Default|GetPlanks)) false))

(fn GeneratePlanks
  (for _index (range 0 (Variables|Default|GetLength))
    (bind _returnvalue (AddComponent|AddStaticMeshComponent false (Math|Transform|MakeTransform (Math|Vector|MakeVector 0.0 (Math|Conversions|ToFloat(Integer) (* _index (Variables|Default|GetGapSize))) 0.0) "0, 0, 0" "1.000000,1.000000,1.000000")))
    (Utilities|Array|Add (Variables|Default|GetPlanks) _returnvalue)))

(fn GenerateConstraints
  (bind _planks (Variables|Default|GetPlanks))
  (for _index (range 0 (- (Variables|Default|GetLength) 1))
    (bind _returnvalue (AddComponent|AddPhysicsConstraintComponent false (Math|Transform|MakeTransform (Math|Vector|MakeVector 0.0 (+ (.y (Variables|/Script/Engine.SceneComponent|GetRelativeLocation (Utilities|Array|Get(acopy) (Variables|Default|GetPlanks) _index))) 3e+01) 0.0) "0.000000,0.000000,90.000000" "1.000000,1.000000,1.000000")))
    (Class|PhysicsConstraintComponent|SetConstrainedComponents _returnvalue (Utilities|Array|Get(acopy) _planks _index) "None" (Utilities|Array|Get(acopy) _planks (+ _index 1)) "None")))