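; Debug trigger actor that unlocks the glide ability and advances checkpoint progress on overlap.
; Any overlap acts on player 0's BP_ThirdPersonCharacter; if glide is off, it enables it, calls the OnGlideEnabled dispatcher and shows its TextRender.
; Separately, if the character's checkpoint string matches PrevCheckpoint, it writes the target string to character and save object, then saves to the character's slot.
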(event Collision|EventActorBeginOverlap
  (params (OtherActor :type Actor%20Object%20Reference))
  (bind _target_checkpoint_progress_string (Variables|Default|GetTarget%20Checkpoint%20Progress%20String))
  (bind _asbp_third_person_character (Utilities|Casting|CastToBP_ThirdPersonCharacter (Game|GetPlayerCharacter 0)))
  (if (Variables|/Game/ThirdPerson/Blueprints/BP_ThirdPersonCharacter.BP_ThirdPersonCharacter_C|GetAbility_Glide _asbp_third_person_character)
    _
    (else
      (Variables|/Game/ThirdPerson/Blueprints/BP_ThirdPersonCharacter.BP_ThirdPersonCharacter_C|SetAbility_Glide _asbp_third_person_character true)
      (Default|CallOnGlideEnabled)
      (Rendering|SetVisibility (Variables|Default|GetTextRender) true false)))
  (if (Utilities|Enum|Equal(Enum) (Variables|/Game/ThirdPerson/Blueprints/BP_ThirdPersonCharacter.BP_ThirdPersonCharacter_C|GetCheckpointProgressString _asbp_third_person_character) (Variables|Default|GetPrevCheckpoint))
    (Variables|/Game/ThirdPerson/Blueprints/BP_ThirdPersonCharacter.BP_ThirdPersonCharacter_C|SetCheckpointProgressString _asbp_third_person_character _target_checkpoint_progress_string)
    (Variables|/Game/ThirdPerson/Maps/BP_Save.BP_Save_C|SetCheckpointProgressString (Variables|/Game/ThirdPerson/Blueprints/BP_ThirdPersonCharacter.BP_ThirdPersonCharacter_C|GetBP_Save _asbp_third_person_character) _target_checkpoint_progress_string)
    (SaveGame|SaveGametoSlot (Variables|/Game/ThirdPerson/Blueprints/BP_ThirdPersonCharacter.BP_ThirdPersonCharacter_C|GetBP_Save _asbp_third_person_character) (Variables|/Game/ThirdPerson/Blueprints/BP_ThirdPersonCharacter.BP_ThirdPersonCharacter_C|GetSaveName _asbp_third_person_character))))

(fn ConstructionScript)