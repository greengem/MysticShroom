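; Debug trigger actor that unlocks the player's double jump ability when overlapped.
; On any actor overlap, it enables the ability on player 0's BP_ThirdPersonCharacter if not already set and calls the OnDoubleJumpEnabled dispatcher.
; It also advances checkpoint progress from 1 to 2, writing it to the character's save object and saving to slot.
; The overlapping actor itself is never checked.
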(event Collision|EventActorBeginOverlap
  (params (OtherActor :type Actor%20Object%20Reference))
  (bind _asbp_third_person_character (Utilities|Casting|CastToBP_ThirdPersonCharacter (Game|GetPlayerCharacter 0)))
  (if (Variables|/Game/ThirdPerson/Blueprints/BP_ThirdPersonCharacter.BP_ThirdPersonCharacter_C|GetAbility_DoubleJump _asbp_third_person_character)
    _
    (else
      (Variables|/Game/ThirdPerson/Blueprints/BP_ThirdPersonCharacter.BP_ThirdPersonCharacter_C|SetAbility_DoubleJump _asbp_third_person_character true)
      (Default|CallOnDoubleJumpEnabled)))
  (if (== (Variables|/Game/ThirdPerson/Blueprints/BP_ThirdPersonCharacter.BP_ThirdPersonCharacter_C|GetCheckpointProgress _asbp_third_person_character) 1)
    (Variables|/Game/ThirdPerson/Blueprints/BP_ThirdPersonCharacter.BP_ThirdPersonCharacter_C|SetCheckpointProgress _asbp_third_person_character 2)
    (Variables|/Game/ThirdPerson/Maps/BP_Save.BP_Save_C|SetCheckpointProgress (Variables|/Game/ThirdPerson/Blueprints/BP_ThirdPersonCharacter.BP_ThirdPersonCharacter_C|GetBP_Save _asbp_third_person_character) 2)
    (SaveGame|SaveGametoSlot (Variables|/Game/ThirdPerson/Blueprints/BP_ThirdPersonCharacter.BP_ThirdPersonCharacter_C|GetBP_Save _asbp_third_person_character) (Variables|/Game/ThirdPerson/Blueprints/BP_ThirdPersonCharacter.BP_ThirdPersonCharacter_C|GetSaveName _asbp_third_person_character))))

(fn ConstructionScript)