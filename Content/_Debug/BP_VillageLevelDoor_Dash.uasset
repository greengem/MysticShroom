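; BP_VillageLevelDoor_Dash is a door actor that opens by snapping 500 units downward.
; Shortly after BeginPlay it opens if the third-person character's CheckpointProgress is at least 5.
; It also binds to the used-glide event on the BP_Teleport_Glide actor it finds in the level, so that event opens it too.
; OpenDoor has no guard, so each call lowers the door again.
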(event Custom|DoorIsOpened
  (CallFunction|OpenDoor))

(event EventBeginPlay
  (Utilities|FlowControl|Delay 0.2)
  (bind _asbp_third_person_character (Utilities|Casting|CastToBP_ThirdPersonCharacter (Game|GetPlayerCharacter 0)))
  (if (>= (Variables|/Game/ThirdPerson/Blueprints/BP_ThirdPersonCharacter.BP_ThirdPersonCharacter_C|GetCheckpointProgress _asbp_third_person_character) 5)
    (CallFunction|OpenDoor))
  (bind _returnvalue (Actor|GetActorOfClass "/Game/Portal/BP_Teleport_Glide.BP_Teleport_Glide_C"))
  (EventDispatchers|BindEventtoTelportUsedGlide _returnvalue (delegate Custom|DoorIsOpened)))

(fn ConstructionScript)

(fn OpenDoor
  (bind _returnvalue (Transformation|GetActorLocation))
  (Transformation|SetActorLocation (Math|Vector|MakeVector (.x _returnvalue) (.y _returnvalue) (- (.z _returnvalue) 5e+02)) false false))