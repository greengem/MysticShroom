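; Village door actor for the Glide level that opens by instantly dropping 500 units.
; Shortly after BeginPlay it reads the player character's checkpoint progress string and opens if that is none of the Spawn or Level1 checkpoints.
; Otherwise it binds to the first teleporter tagged Teleport_Jump and opens when that teleporter's used event reports Glide as the door to unlock.
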(event Custom|CustomEvent
  (params (DoorToUnlock :type String))
  (if (Utilities|Enum|Equal(Enum) DoorToUnlock "Glide")
    (CallFunction|OpenDoor)))

(event EventBeginPlay
  (Utilities|FlowControl|Delay 0.2)
  (bind _asbp_third_person_character (Utilities|Casting|CastToBP_ThirdPersonCharacter (Game|GetPlayerCharacter 0)))
  (if (Math|Boolean|ANDBoolean (Utilities|Enum|NotEqual(Enum) (Variables|/Game/ThirdPerson/Blueprints/BP_ThirdPersonCharacter.BP_ThirdPersonCharacter_C|GetCheckpointProgressString _asbp_third_person_character) "Spawn") (Utilities|Enum|NotEqual(Enum) (Variables|/Game/ThirdPerson/Blueprints/BP_ThirdPersonCharacter.BP_ThirdPersonCharacter_C|GetCheckpointProgressString _asbp_third_person_character) "Level1Start") (Utilities|Enum|NotEqual(Enum) (Variables|/Game/ThirdPerson/Blueprints/BP_ThirdPersonCharacter.BP_ThirdPersonCharacter_C|GetCheckpointProgressString _asbp_third_person_character) "Level1AbilityUnlock") (Utilities|Enum|NotEqual(Enum) (Variables|/Game/ThirdPerson/Blueprints/BP_ThirdPersonCharacter.BP_ThirdPersonCharacter_C|GetCheckpointProgressString _asbp_third_person_character) "Level1Complete"))
    (CallFunction|OpenDoor)
    (else
      (bind _outactors (Actor|GetAllActorsOfClasswithTag "/Game/Portal/BP_Teleport.BP_Teleport_C" "Teleport_Jump"))
      (EventDispatchers|BindEventtoTelportUsed (Utilities|Array|Get(acopy) _outactors) (delegate Custom|CustomEvent)))))

(fn ConstructionScript)

(fn OpenDoor
  (bind _returnvalue (Transformation|GetActorLocation))
  (Transformation|SetActorLocation (Math|Vector|MakeVector (.x _returnvalue) (.y _returnvalue) (- (.z _returnvalue) 5e+02)) false false))