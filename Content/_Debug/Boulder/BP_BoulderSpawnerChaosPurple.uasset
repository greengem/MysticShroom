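; Debug spawner actor that repeatedly spawns purple rolling boulders (BP_BoulderRollingPurple) at its own transform.
; BeginPlay starts a looping timer whose random 5–15 second interval is picked once.
; Each spawn is added to SpawnedBoulders and the indexed entry is passed to KillBoulder, which waits, then increments IndexCount.
; The DestroyActor call is never executed, so this spawner removes no boulders.
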(event Custom|SpawnBoulder
  (bind _spawnedboulders (Variables|Default|GetSpawnedBoulders))
  (Game|SpawnActorfromClass "/Game/_Debug/Boulder/BP_BoulderRollingPurple.BP_BoulderRollingPurple_C" (Transformation|GetActorTransform) "Undefined" "MultiplyWithRoot" 0 0)
  (Utilities|Array|Add _spawnedboulders 0)
  (CallFunction|KillBoulder (Utilities|Array|Get(acopy) _spawnedboulders (Variables|Default|GetIndexCount))))

(event Custom|Kill%20Boulder
  (params (Target :type Actor%20Object%20Reference))
  (Utilities|FlowControl|Delay 2e+01)
  (bind _result (Math|Integer|IncrementInt (Variables|Default|GetIndexCount))
    (:%20%20
      (Variables|Default|SetIndexCount _result))))

(event EventBeginPlay
  (Utilities|Time|SetTimerbyEvent (delegate Custom|SpawnBoulder) (Math|Random|RandomFloatinRange 5.0 15.0) true))

(fn ConstructionScript)